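; BP_Audio is an actor that plays, back to back, the audio supplied by the WBPInputText widget, within the XGXunFei Talk feature.
; It fetches the widget's current audio into its Audio component, retrying every tick while the widget or sound is invalid.
; OnAudioFinished restarts the fetch, forming a continuous playback loop.
; Tick independently yaws the root component at RotateRate, scaled by delta time.
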(event OnAudioFinished(Audio)
  (CallFunction|StartAudio))

(event Custom|StartAudio
  (bind _wbp_inputtext (Variables|Default|GetWBP_InputText))
  (bind _audio (Variables|Default|GetAudio))
  (Utilities|IsValid _wbp_inputtext
    (:Is%20Valid
      (bind _outaudio (Default|GetCurrentAudio _wbp_inputtext))
      (Utilities|IsValid _outaudio
        (:Is%20Valid
          (Variables|/Script/Engine.AudioComponent|SetSound _audio _outaudio)
          (Audio|Components|Audio|Play _audio 0.0))
        (:Is%20Not%20Valid
          (Utilities|FlowControl|DelayUntilNextTick :!label _label)
          (CallFunction|StartAudio))))
    (:Is%20Not%20Valid
      (goto _label))))

(event EventTick
  (params (DeltaSeconds :type Float%20%28single-precision%29))
  (Transformation|AddWorldRotation (Variables|Default|GetDefaultSceneRoot) (Math|Rotator|MakeRotator 0.0 0.0 (* DeltaSeconds (Variables|Default|GetRotateRate))) false false))

(event EventBeginPlay
  (CallFunction|StartAudio))

(fn ConstructionScript)