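; Blueprint function library for the XunFei talk framework, providing talk HUD lookup and splitting of Spark message strings.
; GetTalkHUD returns a player controller's HUD cast to BP_TalkHUD.
; ParseSparkString splits a message just past the first character of a found substring.
; BatchParseSparkString tries this against a substring list and returns the first match in list order, not necessarily the earliest in the text.
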(fn GetTalkHUD
  (params (InPlayerController :type Player%20Controller%20Object%20Reference))
  (bind _returnvalue (HUD|GetHUD InPlayerController))
  (Utilities|IsValid InPlayerController
    (:Is%20Valid
      (Utilities|IsValid _returnvalue
        (:Is%20Valid
          (bind _asbp_talk_hud (Utilities|Casting|CastToBP_TalkHUD _returnvalue))
          (return _asbp_talk_hud))))))

(fn ParseSparkString
  (params (InMessage :type String) (InSubstring :type String))
  (bind _returnvalue (Utilities|String|MakeLiteralString InMessage))
  (bind _returnvalue_2 (Utilities|String|FindSubstring _returnvalue InSubstring))
  (bind _returnvalue_3 (+ _returnvalue_2 1))
  (if (!= _returnvalue_2 -1)
    (return true (Utilities|String|Left _returnvalue _returnvalue_3) (Utilities|String|RightChop _returnvalue _returnvalue_3))
    (else
      (return false "" ""))))

(fn BatchParseSparkString
  (params (InMessage :type String) (__WorldContext :type Object%20Object%20Reference))
  (for _array_element (LocalVariables|GetSubstrings)
    (if (.bParse (CallFunction|ParseSparkString InMessage _array_element __WorldContext))
      (return true (.LeftString (CallFunction|ParseSparkString InMessage _array_element __WorldContext)) (.RightString (CallFunction|ParseSparkString InMessage _array_element __WorldContext)))))
  (return false "" ""))